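; BP_Effect is an effect actor that animates the material on its static mesh by stepping a frame index.
; On BeginPlay it creates a dynamic material instance from slot 0 and starts a looping one-second timer.
; Each tick of that timer writes AnimationIndex to the material's scalar parameter of the same name, then increments it without wrapping, leaving any visual change to the material.
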(event `self.ReceiveBeginPlay`
  (bind _returnvalue (`PrimitiveComponent.CreateDynamicMaterialInstance` (`self.StaticMesh`) 0 (`PrimitiveComponent.GetMaterial` (`self.StaticMesh`) 0) "None"))
  (bind _output_get (set `self.NewVar` _returnvalue))
  (`KismetSystemLibrary.K2_SetTimerDelegate` (delegate `カスタムイベント`) 1.0 true))

(event `カスタムイベント`
  (`MaterialInstanceDynamic.SetScalarParameterValue` (`self.NewVar`) "AnimationIndex" (`KismetMathLibrary.Conv_IntToDouble` (`self.AnimationIndex`)))
  (`/Engine/EditorBlueprintResources/StandardMacros.IncrementInt` (`self.AnimationIndex`)))

(fn `UserConstructionScript`)